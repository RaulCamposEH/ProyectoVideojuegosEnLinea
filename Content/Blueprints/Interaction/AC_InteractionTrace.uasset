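; Interaction component that lets the player focus and use BP_InteractionArea objects by looking at them.
; Each tick, a visibility line trace along the camera direction toggles focus on the hit area.
; TryToInteract fires InteractOnServer immediately for zero-duration areas, or runs a looping timer that fills the WB_Interaction progress widget.
; Completed holds message the area's parent to interact and be destroyed and set PickedUp, while release or focus loss resets progress.
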(event `self.ReceiveTick`
  (params (DeltaSeconds :type "Float (single-precision)"))
  (`self.Trace`))

(event `TryToInteract`
  (params (In :type Boolean))
  (if In
    (if (`self.isTracingInteractionArea`)
      (bind _output_get (set `self.Interact Duration` (`/Game/Blueprints/Interaction/InteractionArea/BP_InteractionArea.Interact Duration` (`self.FocusedInteractionArea`))))
      (if (> _output_get 0.0)
        (bind _ref (message `/Game/Blueprints/Interaction/BI_Interaction.GetInteractionWidgetRef` (`Actor.GetParentActor` (`self.FocusedInteractionArea`))))
        (bind _aswb_interaction (cast `/Game/Blueprints/Interaction/WB_Interaction` (`WidgetComponent.GetWidget` _ref)))
        (set `self.Current_InteractW_REF` _aswb_interaction)
        (bind _returnvalue (`KismetSystemLibrary.K2_SetTimerDelegate` (delegate `Update Interaction Progress`) (`self.Update_Interval`) true))
        (set `self.InteractionTimer` _returnvalue)
        (else
          (`self.InteractOnServer` (`self.FocusedInteractionArea`)))))
    (else
      (`self.StopInteraction`))))

(event `InteractOnServer`
  (params (InteractionArea :type "/Game/Blueprints/Interaction/InteractionArea/BP_InteractionArea Object Reference"))
  (message `/Game/Blueprints/Interaction/BI_Interaction.Interface_Interact` (`Actor.GetParentActor` InteractionArea)))

(event `Update Interaction Progress`
  (bind _output_get (set `self.Interaction_progress` (+ (`self.Interaction_progress`) (* (/ 1.0 (`self.Interact Duration`)) (`self.Update_Interval`)))))
  (`/Game/Blueprints/Interaction/WB_Interaction.setPercent` (`self.Current_InteractW_REF`) _output_get)
  (if (>= (`self.Interaction_progress`) 1.0)
    (`self.StopInteraction`)
    (`self.InteractOnServer` (`self.FocusedInteractionArea`))
    (`self.RunEventAfterInteraction` false)
    (set `self.pickedUp` true)
    (`self.DestroyInteractionArea` (`self.FocusedInteractionArea`))))

(event `DestroyInteractionArea`
  (params (DestroyTarget :type "/Game/Blueprints/Interaction/InteractionArea/BP_InteractionArea Object Reference"))
  (message `/Game/Blueprints/Interaction/BI_Interaction.Interface_Destroy` (`Actor.GetParentActor` DestroyTarget)))

(fn `getPickedUp`
  (returns (PickedUp :type Boolean))
  (return (`self.pickedUp`)))

(fn `RunEventAfterInteraction`
  (params (destroyed :type Boolean))
  (locals (ParentActor :type "Actor Object Reference"))
  (set `local.ParentActor` (`Actor.GetParentActor` (`self.FocusedInteractionArea`)))
  (set `self.isTracingInteractionArea` false)
  (cast `/Game/ThirdPerson/Blueprints/BP_Character` (`GameplayStatics.GetPlayerPawn` 0)
    (:`then`
      (`KismetSystemLibrary.PrintText` "Yes"))
    (:`CastFailed`
      (`KismetSystemLibrary.PrintText` "no"))))

(fn `StopInteraction`
  (if (> (`self.Interaction_progress`) 0.0)
    (`KismetSystemLibrary.K2_ClearAndInvalidateTimerHandle` (`self.InteractionTimer`))
    (`/Game/Blueprints/Interaction/WB_Interaction.setPercent` (`self.Current_InteractW_REF`) 0.0)
    (set `self.Interaction_progress` 0.0)
    (set `self.Current_InteractW_REF` null)))

(fn `Trace`
  (bind _returnvalue (`SceneComponent.K2_GetComponentLocation` (`self.OriginActor`)))
  (bind (_outhit _returnvalue_2) (`KismetSystemLibrary.LineTraceSingle` _returnvalue (+ _returnvalue (* (`KismetMathLibrary.GetForwardVector` (`Actor.K2_GetActorRotation` (`GameplayStatics.GetPlayerCameraManager` 0))) (`self.lenght`))) "TraceTypeQuery1"))
  (if _returnvalue_2
    (bind (_bblockinghit _binitialoverlap _time _distance _location _impactpoint _normal _impactnormal _physmat _hitactor) (`GameplayStatics.BreakHitResult` _outhit))
    (if (!= (`self.FocusedActor`) _hitactor)
      (set `self.FocusedActor` _hitactor)
      (bind _returnvalue_3 (`GameplayStatics.GetObjectClass` _hitactor))
      (`self.TraceInteractionArea` (or (== _returnvalue_3 "/Game/Blueprints/Interaction/InteractionArea/BP_InteractionArea_Box.BP_InteractionArea_Box_C") (== _returnvalue_3 "/Game/Blueprints/Interaction/InteractionArea/BP_InteractionArea_CustomShape.BP_InteractionArea_CustomShape_C"))))
    (else
      (`self.TraceInteractionArea` false))))

(fn `TraceInteractionArea`
  (params (Trace :type Boolean))
  (if Trace
    (if (`self.isTracingInteractionArea`)
      (`/Game/Blueprints/Interaction/InteractionArea/BP_InteractionArea.ToggleFocus` (`self.FocusedInteractionArea`) false))
    (bind _asbp_interaction_area (cast `/Game/Blueprints/Interaction/InteractionArea/BP_InteractionArea` (`self.FocusedActor`)))
    (bind _output_get (set `self.FocusedInteractionArea` _asbp_interaction_area))
    (`/Game/Blueprints/Interaction/InteractionArea/BP_InteractionArea.ToggleFocus` _output_get true)
    (set `self.isTracingInteractionArea` true)
    (elif (`self.isTracingInteractionArea`)
      (set `self.isTracingInteractionArea` false)
      (`/Game/Blueprints/Interaction/InteractionArea/BP_InteractionArea.ToggleFocus` (`self.FocusedInteractionArea`) false)
      (set `self.FocusedActor` null)
      (set `self.FocusedInteractionArea` null)
      (`self.StopInteraction`))))