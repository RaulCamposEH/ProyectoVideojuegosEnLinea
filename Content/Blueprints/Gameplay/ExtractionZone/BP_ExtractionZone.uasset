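; Extraction zone actor that lets a character carrying the winning object win by staying inside its overlap area.
; Entering stores the character and starts a looping timer that builds extraction progress at a rate based on the tick interval.
; Leaving with the object clears the timer and resets any progress made.
; Full progress flags the player's BP_PS_Extraction state as winner and calls EnviarPuntajes (send scores) once.
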(event `TryToExtract`
  (params (In :type Boolean))
  (if In
    (bind _returnvalue (`KismetSystemLibrary.K2_SetTimerDelegate` (delegate `Update Extraction Progress`) (`self.Time`) true))
    (set `self.Timer` _returnvalue)
    (else
      (`self.Stop Extraction`))))

(event `self.ReceiveActorBeginOverlap`
  (params (OtherActor :type "Actor Object Reference"))
  (bind _asbp_character (cast `/Game/Character_Final/BP_Character` OtherActor))
  (set `self.BP Character` _asbp_character)
  (if (`/Game/Character_Final/BP_Character.Has Winning Object` _asbp_character)
    (`self.TryToExtract` true)))

(event `Update Extraction Progress`
  (bind _bp_character (`self.BP Character`))
  (bind _output_get (set `self.Extraction progress` (+ (`self.Extraction progress`) (* (/ 1.0 10.0) (`self.Time`)))))
  (if (>= _output_get 1.0)
    (bind _asbp_ps_extraction (cast `/Game/Character_Final/BP_PS_Extraction` (`Pawn.PlayerState` _bp_character)))
    (set `/Game/Character_Final/BP_PS_Extraction.Winner` true _asbp_ps_extraction)
    (`/Engine/EditorBlueprintResources/StandardMacros.DoOnce` false
      (:`Completed`
        (`/Game/Character_Final/BP_Character.EnviarPuntajes` _bp_character)))))

(event `self.ReceiveActorEndOverlap`
  (params (OtherActor :type "Actor Object Reference"))
  (bind _asbp_character (cast `/Game/Character_Final/BP_Character` OtherActor))
  (if (`/Game/Character_Final/BP_Character.Has Winning Object` _asbp_character)
    (`self.TryToExtract` false)))

(fn `Stop Extraction`
  (if (> (`self.Extraction progress`) 0.0)
    (`KismetSystemLibrary.K2_ClearAndInvalidateTimerHandle` (`self.Timer`))
    (set `self.Extraction progress` 0.0)))

(fn `UserConstructionScript`)