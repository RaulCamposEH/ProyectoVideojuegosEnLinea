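; Weapon_BP is a usable weapon that spawns an actor when its Action event fires with a rotator.
; Action passes the rotator to ShootWeapon, which rotates an Offset vector by it and adds that to the Arrow component's world location to push the spawn point forward.
; The actor spawns there facing the rotator, and the computed location is printed as debug output.
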(event `/Game/Blueprints/Gameplay/Usables/BPI_Usable.Action`
  (params (Rotator :type "Rotator Structure"))
  (`self.ShootWeapon` Rotator))

(fn `ShootWeapon`
  (params (Rotator :type "Rotator Structure"))
  (bind _returnvalue (+ (`SceneComponent.K2_GetComponentLocation` (`self.Arrow`)) (`KismetMathLibrary.GreaterGreater_VectorRotator` (`self.offset`) Rotator)))
  (`KismetSystemLibrary.PrintString` (`KismetStringLibrary.Conv_VectorToString` _returnvalue))
  (`|SpawnActorFromClass` "/Game/Blueprints/Bullet_Damage.Bullet_Damage_C" (`KismetMathLibrary.MakeTransform` _returnvalue Rotator) "Undefined" "OverrideRootScale" null null))

(fn `UserConstructionScript`)