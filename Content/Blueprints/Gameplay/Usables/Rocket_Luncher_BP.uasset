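; Rocket launcher usable Blueprint that fires a projectile when its Action event runs.
; ShootRocket spawns an Explosion_Damage actor at the skeletal mesh's spawn socket, pushed forward by an offset rotated into camera space.
; The spawned actor faces the rotation of player 0's camera manager, which avoids hard references to the owning character.
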(event `/Game/Blueprints/Gameplay/Usables/BPI_Usable.Action`
  (`self.ShootRocket`))

(fn `ShootRocket`
  (bind _returnvalue (`PlayerCameraManager.GetCameraRotation` (`GameplayStatics.GetPlayerCameraManager` 0)))
  (`|SpawnActorFromClass` "/Game/Blueprints/Explosion_Damage.Explosion_Damage_C" (`KismetMathLibrary.MakeTransform` (+ (`SceneComponent.GetSocketLocation` (`self.SkeletalMesh`) (`self.Socket Spawn`)) (`KismetMathLibrary.GreaterGreater_VectorRotator` (`self.offset`) _returnvalue)) _returnvalue) "Undefined" "OverrideRootScale" null null))

(fn `UserConstructionScript`)