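; Projectile that damages whatever it hits and leaves a BP_MasterField actor at the impact point.
; On hit, Impact spawns that field once through a DoOnce-guarded event and pushes physics-simulating components with an impulse scaled from the bullet's velocity.
; It then plays a smoke explosion effect, applies fixed damage to the hit actor and destroys itself.
; A debug sphere draw is present but disabled.
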(event `SpawnMaster`
  (params (Location :type "Vector Structure"))
  (`/Engine/EditorBlueprintResources/StandardMacros.DoOnce` false
    (:`Completed`
      (`|SpawnActorFromClass` "/Game/Blueprints/Destruibles/BP_MasterField.BP_MasterField_C" (`KismetMathLibrary.MakeTransform` Location) "Undefined" "OverrideRootScale" null null))))

(event `self.ReceiveHit`
  (params (MyComp :type "PrimitiveComponent Object Reference") (Other :type "Actor Object Reference") (OtherComp :type "PrimitiveComponent Object Reference") (bSelfMoved :type Boolean) (HitLocation :type "Vector Structure") (HitNormal :type "Vector Structure") (NormalImpulse :type "Vector Structure") (Hit :type "HitResult Structure (by ref)"))
  (`self.Impact` OtherComp HitLocation Other))

(fn `Impact`
  (params (InputPin :type "PrimitiveComponent Object Reference") (Location :type "Vector Structure") (DamagedActor :type "Actor Object Reference"))
  (locals (LocalLocation :type "Vector Structure") (damaged :type "Actor Object Reference"))
  (set `local.LocalLocation` Location)
  (set `local.damaged` DamagedActor)
  (`self.SpawnMaster` (`local.LocalLocation`))
  (if (`SceneComponent.IsSimulatingPhysics` InputPin "None")
    (`PrimitiveComponent.AddImpulseAtLocation` InputPin (* (`self.GetVelocity`) 100.0) (`self.K2_GetActorLocation`) "None"))
  (`GameplayStatics.SpawnEmitterAtLocation` "/Game/Assets/Particulas/Explosion/P_Explosion_Smoke.P_Explosion_Smoke" (`local.LocalLocation`) (struct) (0.5 0.5 0.5))
  (if false
    (`KismetSystemLibrary.DrawDebugSphere` (`local.LocalLocation`) 600.0 12 (struct :`R` 1.0 :`A` 1.0) 3.0 5.0))
  (`GameplayStatics.ApplyDamage` (`local.damaged`) 20.0)
  (`self.K2_DestroyActor`) ; Then destroy this projectile
)

(fn `UserConstructionScript`)