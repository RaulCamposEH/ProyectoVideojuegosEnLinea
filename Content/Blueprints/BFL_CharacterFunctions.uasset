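; Blueprint function library of character helpers for cycling integer-style values and initializing an IT component.
; ScrollUp and ScrollDown step a value by one and wrap it to the opposite bound when it passes Min or Max.
; SetupIT hands an origin skeletal mesh and origin character to the IT component, then enables that component's tick.
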(fn `ScrollDown`
  (params (Value :type Integer) (Min :type Integer) (Max :type Integer))
  (returns (Return :type Integer))
  (locals (LocalValue :type Integer))
  (bind _returnvalue (- Value 1))
  (if (< _returnvalue Min)
    (set `local.LocalValue` Max)
    (else
      (set `local.LocalValue` _returnvalue)))
  (return (`local.LocalValue`)))

(fn `ScrollUp`
  (params (Value :type Integer) (Min :type Integer) (Max :type Integer))
  (returns (Return :type Integer))
  (locals (LocalValue :type Integer))
  (bind _returnvalue (+ Value 1))
  (if (> _returnvalue Max)
    (set `local.LocalValue` Min)
    (else
      (set `local.LocalValue` _returnvalue)))
  (return (`local.LocalValue`)))

(fn `SetupIT`
  (params (OriginSKM :type "SkeletalMeshComponent Object Reference") (ITComponent :type "/Game/Blueprints/Interaction/AC_InteractionTrace Object Reference") (`Origin Char` :type "/Game/ThirdPerson/Blueprints/BPI_CharacterInteract Interface"))
  (set `/Game/Blueprints/Interaction/AC_InteractionTrace.OriginSKM` OriginSKM ITComponent)
  (set `/Game/Blueprints/Interaction/AC_InteractionTrace.OriginCharacter` `Origin Char` ITComponent)
  (`ActorComponent.SetComponentTickEnabled` ITComponent true))