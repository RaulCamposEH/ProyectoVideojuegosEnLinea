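; Projectile Blueprint that explodes on hit, dealing radial damage with falloff, then destroys itself.
; The Hit event calls Explode, which pushes physics-simulating components with a velocity-based impulse and plays an explosion emitter.
; Explode also calls SpawnMaster, whose DoOnce gate limits it to spawning one scaled-up BP_MasterField at the impact point.
; A debug sphere matching the damage radius is present but disabled.
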(event `SpawnMaster`
  (params (Location :type "Vector Structure"))
  (`/Engine/EditorBlueprintResources/StandardMacros.DoOnce` false
    (:`Completed`
      (`|SpawnActorFromClass` "/Game/Blueprints/Destruibles/BP_MasterField.BP_MasterField_C" (`KismetMathLibrary.MakeTransform` Location (struct) (5.0 5.0 5.0)) "Undefined" "OverrideRootScale" null null))))

(event `self.ReceiveHit`
  (params (MyComp :type "PrimitiveComponent Object Reference") (Other :type "Actor Object Reference") (OtherComp :type "PrimitiveComponent Object Reference") (bSelfMoved :type Boolean) (HitLocation :type "Vector Structure") (HitNormal :type "Vector Structure") (NormalImpulse :type "Vector Structure") (Hit :type "HitResult Structure (by ref)"))
  (`self.Explode` OtherComp HitLocation))

(fn `Explode`
  (params (Component :type "PrimitiveComponent Object Reference") (Location :type "Vector Structure"))
  (locals (NewLocalVar :type "Vector Structure" :default (0.0 0.0 0.0)) (LocalLocation :type "Vector Structure" :default (0.0 0.0 0.0)))
  (set `local.LocalLocation` Location)
  (`self.SpawnMaster` (`local.LocalLocation`))
  (if (`SceneComponent.IsSimulatingPhysics` Component "None")
    (`PrimitiveComponent.AddImpulseAtLocation` Component (* (`self.GetVelocity`) 200.0) (`self.K2_GetActorLocation`) "None"))
  (`GameplayStatics.SpawnEmitterAtLocation` "/Game/Realistic_Starter_VFX_Pack_Vol2/Particles/Explosion/P_Explosion_Big_C.P_Explosion_Big_C" (`local.LocalLocation`) (struct) (1.5 0.5 0.5))
  (if false
    (`KismetSystemLibrary.DrawDebugSphere` (`local.LocalLocation`) 600.0 12 (struct :`R` 1.0 :`A` 1.0) 3.0 5.0))
  (`GameplayStatics.ApplyRadialDamageWithFalloff` :`BaseDamage` 110.0 :`MinimumDamage` 20.0 :`Origin` (`local.LocalLocation`) :`DamageOuterRadius` 600.0 :`DamageFalloff` 0.5 :`DamageCauser` null :`InstigatedByController` null)
  (`self.K2_DestroyActor`) ; Then destroy this projectile
)

(fn `UserConstructionScript`)