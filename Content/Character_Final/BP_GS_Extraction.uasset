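; Game state for the Extraction mode that relays pause, victory-list and player-window events across the player array.
; These three events act only on the Remote branch, using array indices to reach each character's PauseAllOnServer and each controller's AbrirVentana.
; The victory event refreshes all top-level victory widgets once per player.
; Update_PlayerList reassigns PlayerArray to itself, and the OnRep handler is empty, with a disconnected copy of the pause loop.
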(event `Update_PlayerList`
  (set `self.Player Array` (`self.PlayerArray`)))

(event `Pauseforallgs`
  (`/Engine/EditorBlueprintResources/ActorMacros.Switch Has Authority`
    (:`Remote`
      (for (_array_element _array_index) (`self.PlayerArray`)
        (`KismetSystemLibrary.PrintString` (`KismetStringLibrary.Conv_IntToString` _array_index))
        (bind _asbp_character (cast `/Game/Character_Final/BP_Character` (`GameplayStatics.GetPlayerCharacter` _array_index)))
        (`/Game/Character_Final/BP_Character.PauseAllOnServer` _asbp_character _array_index))
      (`KismetSystemLibrary.PrintString` (`PlayerState.GetPlayerName` _array_element)))))

(event `listavictoria`
  (`/Engine/EditorBlueprintResources/ActorMacros.Switch Has Authority`
    (:`Remote`
      (for _ (`self.PlayerArray`)
        (bind _foundwidgets (`WidgetBlueprintLibrary.GetAllWidgetsOfClass` "/Game/UiUx/WI_VICTORIA/W_BP_VICTORIA.W_BP_VICTORIA_C"))
        (for _array_element _foundwidgets
          (`/Game/UiUx/WI_VICTORIA/W_BP_VICTORIA.Update_Widget` _array_element))))))

(event `abrir_lista_pc`
  (`/Engine/EditorBlueprintResources/ActorMacros.Switch Has Authority`
    (:`Remote`
      (for (_ _array_index) (`self.PlayerArray`)
        (bind _asbp_pc_extraction (cast `/Game/Character_Final/BP_PC_Extraction` (`GameplayStatics.GetPlayerController` _array_index)))
        (`/Game/Character_Final/BP_PC_Extraction.abrir ventana` _asbp_pc_extraction _array_index)))))

(fn `OnRep_Player Array`)

(fn `UserConstructionScript`)