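; Game mode for the Extraction game that tracks connected players and keeps the game state's player list current.
; Login and logout add or remove the Extraction player controller in an array, then trigger a list update.
; The update waits with a zero-length delay before asking the Extraction game state to refresh its player list.
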(event `self.K2_PostLogin`
  (params (NewPlayer :type "PlayerController Object Reference"))
  (bind _asbp_pc_extraction (cast `/Game/Character_Final/BP_PC_Extraction` NewPlayer))
  (`KismetArrayLibrary.Array_Add` (`self.ALL_PLAYER_CONTROLLER`) _asbp_pc_extraction)
  (`self.Update_Player_List` :!label _label))

(event `Update_Player_List`
  (`KismetSystemLibrary.Delay` 0.0)
  (bind _asbp_gs_extraction (cast `/Game/Character_Final/BP_GS_Extraction` (`GameplayStatics.GetGameState`)))
  (`/Game/Character_Final/BP_GS_Extraction.Update_PlayerList` _asbp_gs_extraction))

(event `self.K2_OnLogout`
  (params (ExitingController :type "Controller Object Reference"))
  (bind _asbp_pc_extraction (cast `/Game/Character_Final/BP_PC_Extraction` ExitingController))
  (`KismetArrayLibrary.Array_RemoveItem` (`self.ALL_PLAYER_CONTROLLER`) _asbp_pc_extraction)
  (goto _label))

(fn `UserConstructionScript`)