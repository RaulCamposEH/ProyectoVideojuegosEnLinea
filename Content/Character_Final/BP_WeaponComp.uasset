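; Weapon component that attaches itself to the owning BP_Character's GunGrip socket and fires bullets.
; The Disparo input fires only while the character is aiming and not reloading, passing camera rotation to ActionOnServer and calling the character's FiringOnServer.
; ActionOnServer relays to ActionOnClient, which spawns Bullet_Damage at the bullet_spawn socket plus a rotated offset and plays the rifle burst sound.
; DestroyUsable removes the component.
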(event `self.ReceiveBeginPlay`
  (bind _asbp_character (cast `/Game/Character_Final/BP_Character` (`self.GetOwner`)))
  (bind _output_get (set `self.BP CharacterRef` _asbp_character))
  (`self.K2_AttachToComponent` (`Character.Mesh` _output_get) "GunGrip" "KeepRelative" "KeepRelative" "KeepRelative"))

(event `EnhancedInput|/Game/Input/Actions/Disparo`
  (params (ActionValue :type Boolean) (ElapsedSeconds :type "Float (double-precision)") (TriggeredSeconds :type "Float (double-precision)") (InputAction :type "InputAction Object Reference" :default "/Game/Input/Actions/Disparo.Disparo"))
  (:`Started`
    (if (and (`/Game/Character_Final/BP_Character.EstaApuntando?` (`self.BP CharacterRef`)) (not (`/Game/Character_Final/BP_Character.reload?` (`self.BP CharacterRef`))))
      (`self.Action On Server` (`PlayerCameraManager.GetCameraRotation` (`GameplayStatics.GetPlayerCameraManager` 0)))
      (`/Game/Character_Final/BP_Character.FiringOnServer` (`self.BP CharacterRef`)))))

(event `Action On Server`
  (params (InputPin :type "Rotator Structure"))
  (`self.ActionOnClient` InputPin))

(event `ActionOnClient`
  (params (InputPin :type "Rotator Structure"))
  (bind _returnvalue (+ (`self.GetSocketLocation` "bullet_spawn") (`KismetMathLibrary.GreaterGreater_VectorRotator` (`self.ProjectileOffset`) InputPin)))
  (`|SpawnActorFromClass` "/Game/Blueprints/Bullet_Damage.Bullet_Damage_C" (`KismetMathLibrary.MakeTransform` _returnvalue InputPin) "Undefined" "OverrideRootScale" null null)
  (`GameplayStatics.PlaySoundAtLocation` "/Game/FPSAssets/Sounds/Sound_Packs/Warfare_SFX_Bundle/Gun_Sound_Essentials/Wavs/Assault_Rifle_Burst.Assault_Rifle_Burst" _returnvalue (struct) 1.0 1.0 0.0 null null null null) ; Play firing sound
)

(event `/Game/Character_Final/BPI_UsableComp.DestroyUsable`
  (`self.K2_DestroyComponent`))