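; Rocket launcher component that attaches to the owning BP_Character's RocketGrip mesh socket and fires missiles.
; The Disparo input, while aiming the bazooka with missiles left, decrements the Misil stat and passes camera rotation through ActionOnServer to ActionOnClient.
; ActionOnClient spawns Explosion_Damage at the bullet_spawn socket, pushed forward by a rotated offset and oriented along the camera.
; DestroyUsable removes the component.
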(event `self.ReceiveBeginPlay`
  (bind _asbp_character (cast `/Game/Character_Final/BP_Character` (`self.GetOwner`)))
  (bind _output_get (set `self.BP CharacterRef` _asbp_character))
  (`self.K2_AttachToComponent` (`Character.Mesh` _output_get) "RocketGrip" "KeepRelative" "KeepRelative" "KeepRelative"))

(event `EnhancedInput|/Game/Input/Actions/Disparo`
  (params (ActionValue :type Boolean) (ElapsedSeconds :type "Float (double-precision)") (TriggeredSeconds :type "Float (double-precision)") (InputAction :type "InputAction Object Reference" :default "/Game/Input/Actions/Disparo.Disparo"))
  (:`Started`
    (if (!= (`.Misil_14_A838826343B88450EE2B179B52427459` (break `/Game/Character_Final/CharacterStats` (`/Game/Character_Final/BP_Character.Character Stats` (`self.BP CharacterRef`)))) 0.0)
      (if (`/Game/Character_Final/BP_Character.BazookaApuntando?` (`self.BP CharacterRef`))
        (setmembers `/Game/Character_Final/CharacterStats` :`StructRef` (`/Game/Character_Final/BP_Character.Character Stats` (`self.BP CharacterRef`)) :`Misil` (- (`.Misil_14_A838826343B88450EE2B179B52427459` (break `/Game/Character_Final/CharacterStats` (`/Game/Character_Final/BP_Character.Character Stats` (`self.BP CharacterRef`)))) 1.0))
        (`self.ActionOnServer` (`PlayerCameraManager.GetCameraRotation` (`GameplayStatics.GetPlayerCameraManager` 0)))))))

(event `ActionOnServer`
  (params (InputPin :type "Rotator Structure"))
  (`self.ActionOnClient` InputPin))

(event `ActionOnClient`
  (params (InputPin :type "Rotator Structure"))
  (`|SpawnActorFromClass` "/Game/Blueprints/Explosion_Damage.Explosion_Damage_C" (`KismetMathLibrary.MakeTransform` (+ (`self.GetSocketLocation` "bullet_spawn") (`KismetMathLibrary.GreaterGreater_VectorRotator` (`self.ProjectileOffset`) InputPin)) InputPin) "Undefined" "OverrideRootScale" null null))

(event `/Game/Character_Final/BPI_UsableComp.DestroyUsable`
  (`self.K2_DestroyComponent`))